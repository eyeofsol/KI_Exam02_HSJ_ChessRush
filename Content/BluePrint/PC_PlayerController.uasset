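; Player controller for a tower defense game that holds the player's health, gold and wave number and handles tower selection.
; BeginPlay initializes those values, and each left click plays a sound, then selects the tower under the mouse or clears the current selection.
; SelectTower deselects the previous tower before selecting a new one.
; ConsumeCost deducts gold, and GameOver pauses the game and replaces all widgets with the game-over panel.
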(event `self.ReceiveBeginPlay`
  (`self.InitSetting`))

(event `Key|LeftMouseButton`
  (params (Key :type "Key Structure"))
  (:`Pressed`
    (`GameplayStatics.PlaySound2D` "/Game/Sound/SQ_Click.SQ_Click" 1.0 1.0 0.0 null null)
    (bind (_isfound _tower) (`/Game/BluePrint/BPFL_Utility.GetTowerUnderMouse`))
    ; 타워 클릭 여부
    (if _isfound
      ; 타워 선택
      (`self.SelectTower` _tower)
      (else
        ; 타워 선택 해제
        (`self.UnSelectTower`)))))

(fn `ConsumeCost`
  (params (Cost :type "Float (double-precision)"))
  ; 소지 골드를 차감
  (set `self.Gold` (- (`self.Gold`) Cost))
  (return))

(fn `GameOver`
  ; 게임을 정지하고 게임오버 패널 출력
  (`GameplayStatics.SetGamePaused` true)
  (`WidgetLayoutLibrary.RemoveAllWidgets`)
  (bind _returnvalue (`|CreateWidget` "/Game/UI/WBP_GameOver.WBP_GameOver_C" (`GameplayStatics.GetPlayerController` 0)))
  (`UserWidget.AddToViewport` _returnvalue 0))

(fn `SelectTower`
  (params (Tower :type "/Game/BluePrint/Tower/BP_TowerBase Object Reference"))
  ; 마우스 아래 타워가 선택한 타워가 아닐 경우
  (if (!= Tower (`self.SelectedTower`))
    ; 기존 선택 타워 해제
    (`self.UnSelectTower`)
    ; 새 타워 선택
    (bind _output_get (set `self.SelectedTower` (`local.Tower`)))
    (`/Game/BluePrint/Tower/BP_TowerBase.Select` _output_get)))

(fn `UnSelectTower`
  ; 선택했던 타워를 해제
  (bind _selectedtower (`self.SelectedTower`)
    (:`then`
      (`/Game/BluePrint/Tower/BP_TowerBase.UnSelect` _selectedtower)
      (set `self.SelectedTower` null))
    (:`else`)))

(fn `UserConstructionScript`)