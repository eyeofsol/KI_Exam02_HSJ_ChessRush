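; Tower manager that places the tower bases and handles mouse-hover highlighting for towers.
; On BeginPlay it spawns a BP_TowerBase slightly above each actor in the TowerLocation array.
; Every Tick, UpdateHighLight queries GetTowerUnderMouse and compares the result with the cached HighLightTower.
; When the target changes, it turns the old tower's highlight off and the new one's on via SetHighLight.
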(event `self.ReceiveBeginPlay`
  (for _array_element (`self.TowerLocation`)
    ; 지정된 타워 스폰 위치에 Base 타워 스폰
    (`|SpawnActorFromClass` "/Game/BluePrint/Tower/BP_TowerBase.BP_TowerBase_C" (`KismetMathLibrary.MakeTransform` (+ (`self.K2_GetActorLocation` _array_element) (0.0 0.0 20.0))) "Undefined" "MultiplyWithRoot" null null)))

(event `self.ReceiveTick`
  (params (DeltaSeconds :type "Float (single-precision)"))
  (`self.UpdateHighLight`))

(fn `UpdateHighLight`
  (locals (NewTower :type "/Game/BluePrint/Tower/BP_TowerBase Object Reference"))
  (bind _newtower (`local.NewTower`))
  (`|ExecutionSequence`
    (:`then_0`
      ; 마우스가 호버링중인 곳에 타워가 있다면 NewTower에 저장
      (bind (_isfound _tower) (`/Game/BluePrint/BPFL_Utility.GetTowerUnderMouse`))
      (if _isfound
        (set `local.NewTower` _tower)))
    (:`then_1`
      (if (!= _newtower (`self.HighLightTower`))
        (`|ExecutionSequence`
          (:`then_0`
            ; 호버링 종료시 하이라이트 제거
            (bind _highlighttower (`self.HighLightTower`)
              (:`then`
                (`/Game/BluePrint/Tower/BP_TowerBase.SetHighLight` _highlighttower false))
              (:`else`)))
          (:`then_1`
            ; 호버링시 하이라이트를 켬
            (bind _output_get (set `self.HighLightTower` _newtower))
            (`/Engine/EditorBlueprintResources/StandardMacros.IsValid` _output_get
              (:`Is Valid`
                (`/Game/BluePrint/Tower/BP_TowerBase.SetHighLight` _output_get true)))))))))

(fn `UserConstructionScript`)