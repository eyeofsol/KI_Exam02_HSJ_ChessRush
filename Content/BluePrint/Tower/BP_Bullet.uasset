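; BP_Bullet is a tower projectile that homes in on a target and damages enemies.
; On BeginPlay, a valid TargetActor's root becomes the ProjectileMovement homing target, and a two-second self-destruct delay starts only in that case.
; On hit it plays a 2D sound, then calls TakeDamage with BulletDamage on BP_EnemyPawn actors tagged Enemy.
; It destroys itself after impact, except when a tagged actor fails the cast.
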(event `self.ReceiveBeginPlay`
  (if (`KismetSystemLibrary.IsValid` (`self.TargetActor`))
    ; 타겟을 받아와 해당 타겟을 유도하며 이동
    (set `ProjectileMovementComponent.HomingTargetComponent` (`Actor.RootComponent` (`self.TargetActor`)) (`self.ProjectileMovement`))
    ; 2초 이상 존재하면 액터 삭제
    (`KismetSystemLibrary.Delay` 2.0)
    (`self.K2_DestroyActor`)))

(event `self.ReceiveHit`
  (params (MyComp :type "PrimitiveComponent Object Reference") (Other :type "Actor Object Reference") (OtherComp :type "PrimitiveComponent Object Reference") (bSelfMoved :type Boolean) (HitLocation :type "Vector Structure") (HitNormal :type "Vector Structure") (NormalImpulse :type "Vector Structure") (Hit :type "HitResult Structure (by ref)"))
  ; 피격 사운드 재생
  (`GameplayStatics.PlaySound2D` "/Game/Sound/BulletHit.BulletHit" 1.0 1.0 0.0 null null)
  ; Hit 대상이 적인지 확인
  (if (`self.ActorHasTag` Other "Enemy")
    ; 적이 맞다면 해당 타겟의 TakeDamage 함수 실행 후 액터 삭제
    (bind _asbp_enemy_pawn (cast `/Game/BluePrint/Enemy/BP_EnemyPawn` Other))
    (`/Game/BluePrint/Enemy/BP_EnemyPawn.TakeDamage` _asbp_enemy_pawn (`self.BulletDamage`))
    (`self.K2_DestroyActor`)
    (else
      ; 타겟이 적이 아니라면 액터 삭제
      (`self.K2_DestroyActor`))))

(fn `UserConstructionScript`)