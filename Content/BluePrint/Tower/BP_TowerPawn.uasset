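; Pawn tower for a tower defense game that shoots enemies and can be upgraded or sold.
; Range overlaps maintain an Enemy-tagged target list and toggle a looping fire timer, while Tick aims FirePoint at the first target for spawned bullets.
; Selection shows the range and spawns an action actor.
; Two upgrade tiers spend gold to improve damage, fire rate and material; selling refunds TowerCost and respawns a tower base.
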(event `self.ReceiveBeginPlay`
  ; 공격 범위 표시 해제
  (`SceneComponent.SetVisibility` (`self.ShowRange`) false false)
  ; 타워 가격 업데이트
  (set `self.TowerCost` (`self.PawnCost`))
  ; 이펙트 실행
  (`ActorComponent.Activate` (`self.SpawnEffect`) true))

(event `self.ReceiveTick`
  (params (DeltaSeconds :type "Float (single-precision)"))
  (`self.SetTargetRotation`))

(event `self.ShotRange.OnComponentBeginOverlap`
  (params (OverlappedComponent :type "PrimitiveComponent Object Reference") (OtherActor :type "Actor Object Reference") (OtherComp :type "PrimitiveComponent Object Reference") (OtherBodyIndex :type Integer) (bFromSweep :type Boolean) (SweepResult :type "HitResult Structure (by ref)"))
  (`self.AddTarget` OtherActor)
  ;[0.15 0.15 0.15 0.5 16] 공격 상태가 아니라면
  (if (not (`self.bIsFire`))
    ; Timer를 이용하여 FireRate마다 Attack 이벤트 발생 후 공격 상태 전환
    (bind _returnvalue (`KismetSystemLibrary.K2_SetTimerDelegate` (`|CreateDelegate` :!event `Attack`) (`self.FireRate`) true))
    (set `self.FireTimer` _returnvalue)
    (set `self.bIsFire` true)))

(event `self.ShotRange.OnComponentEndOverlap`
  (params (OverlappedComponent :type "PrimitiveComponent Object Reference") (OtherActor :type "Actor Object Reference") (OtherComp :type "PrimitiveComponent Object Reference") (OtherBodyIndex :type Integer))
  (`self.RemoveTarget` OtherActor)
  ; 타이머 핸들 초기화 및 공격 상태 해제
  (`KismetSystemLibrary.K2_ClearAndInvalidateTimerHandle` (`self.FireTimer`))
  (set `self.bIsFire` false))

(event `Attack`
  ; 총알을 스폰하여 공격 위치와 공격할 타겟을 전달
  (bind _returnvalue (`|SpawnActorFromClass` "/Game/BluePrint/Tower/BP_Bullet.BP_Bullet_C" (`SceneComponent.K2_GetComponentToWorld` (`self.FirePoint`)) "Undefined" "MultiplyWithRoot" null (`|GetArrayItem` (`self.Targets`)) null))
  ; 총알의 데미지를 전달
  (bind _output_get (set `self.Bullet` _returnvalue))
  (set `/Game/BluePrint/Tower/BP_Bullet.BulletDamage` (`self.FireDamage`) _output_get))

(fn `DoTowerAction`
  (params (TowerAction :type "/Game/BluePrint/Tower/E_TowerAction Enum" :default "NewEnumerator0"))
  (bind (_isvalid _aspc_player_controller) (`/Game/BluePrint/BPFL_Utility.GetPlayer`))
  (set `self.PlayerController` _aspc_player_controller)
  (`|ExecutionSequence`
    (:`then_0`
      (bind (_isvalid_2 _aspc_player_controller_2) (`/Game/BluePrint/BPFL_Utility.GetPlayer`))
      (if _isvalid_2
        (`/Game/BluePrint/PC_PlayerController.UnSelectTower` _aspc_player_controller_2)))
    (:`then_1`
      (switch `/Game/BluePrint/Tower/E_TowerAction` TowerAction
        (:`NewEnumerator5`
          (`self.UpgradeTower`))
        (:`NewEnumerator6`
          (`self.SellTower`))))))

(fn `Select`
  ; 해당 타워의 업데이트 위젯을 출력하기 위해 액터를 스폰하고 공격 범위 표시를 전환
  (bind _returnvalue (`|SpawnActorFromClass` "/Game/BluePrint/Tower/BP_PawnTowerUpdate.BP_PawnTowerUpdate_C" (`KismetMathLibrary.MakeTransform` (+ (`self.K2_GetActorLocation`) (0.0 0.0 100.0))) "Undefined" "MultiplyWithRoot" self "NewEnumerator5" "NewEnumerator6" (`self.UpgradeCost`) (`self.TowerCost`) null))
  (set `self.PawnUpdate` _returnvalue)
  (`SceneComponent.SetVisibility` (`self.ShowRange`) true false))

(fn `SellTower`
  (bind _playercontroller (`self.PlayerController`))
  ; 현재 타워의 가격만큼 소지 골드를 추가
  (set `/Game/BluePrint/PC_PlayerController.Gold` (+ (`self.TowerCost`) (`/Game/BluePrint/PC_PlayerController.Gold` _playercontroller)) _playercontroller)
  ; 판매한 타워 위치에 Base타워 생성 후 기존의 타워 제거
  (`|SpawnActorFromClass` "/Game/BluePrint/Tower/BP_TowerBase.BP_TowerBase_C" (`self.GetTransform`) "Undefined" "MultiplyWithRoot" null null)
  (`GameplayStatics.PlaySound2D` "/Game/Sound/SQ_Sell.SQ_Sell" 1.0 1.0 0.0 null null)
  (`self.K2_DestroyActor`))

(fn `UnSelect`
  (bind _pawnupdate (`self.PawnUpdate`)
    (:`then`
      (`self.K2_DestroyActor` _pawnupdate)
      (`SceneComponent.SetVisibility` (`self.ShowRange`) false false))
    (:`else`)))

(fn `UpgradeTower`
  (if (>= (`/Game/BluePrint/PC_PlayerController.Gold` (`self.PlayerController`)) (`self.UpgradeCost`))
    ; 맥스 업그레이드 여부 확인
    (if (`self.IsMax`)
      ; 맥스 업그레이드라면 배너 출력
      (`/Game/UI/WBP_BaseUI.TowerBannerFade` (`self.Widget`))
      (`GameplayStatics.PlaySound2D` "/Game/Sound/SQ_Interupt.SQ_Interupt" 1.0 1.0 0.0 null null)
      (else
        (`GameplayStatics.PlaySound2D` "/Game/Sound/SQ_Build.SQ_Build" 1.0 1.0 0.0 null null)
        ; 업그레이드 상태 확인
        (if (`self.IsUpgrade`)
          ; 업그레이드 상태라면 두 번째 업그레이드 실행
          (`self.UpgradeSecond`)
          (else
            ; 업그레이드 상태가 아니라면 첫 번째 업그레이드 실행
            (`self.UpgradeFirst`)))
        (return)))
    (else
      ; 충분하지 않다면 골드 부족 배너 출력
      (`/Game/UI/WBP_BaseUI.CoinBannerFade` (`self.Widget`))
      (`GameplayStatics.PlaySound2D` "/Game/Sound/SQ_Interupt.SQ_Interupt" 1.0 1.0 0.0 null null))))

(fn `UserConstructionScript`)