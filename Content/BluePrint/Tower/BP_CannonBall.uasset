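; BP_CannonBall is a tower cannonball projectile that deals area damage to enemies on impact.
; Its DamageRange component adds Enemy-tagged actors to Targets as they begin overlapping, with no removal when they leave.
; On any Hit, PlayFX plays a 2D sound and spawns an explosion effect, then the ball destroys itself.
; Only a hit on an enemy applies BulletDamage to the stored targets through BP_EnemyPawn's TakeDamage.
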(event `self.DamageRange.OnComponentBeginOverlap`
  (params (OverlappedComponent :type "PrimitiveComponent Object Reference") (OtherActor :type "Actor Object Reference") (OtherComp :type "PrimitiveComponent Object Reference") (OtherBodyIndex :type Integer) (bFromSweep :type Boolean) (SweepResult :type "HitResult Structure (by ref)"))
  ; 데미지 범위만큼 Overlap된 액터들을 배열에 저장
  (if (`KismetSystemLibrary.IsValid` OtherActor)
    (if (`self.ActorHasTag` OtherActor "Enemy")
      (`KismetArrayLibrary.Array_Add` (`self.Targets`) OtherActor))))

(event `self.ReceiveHit`
  (params (MyComp :type "PrimitiveComponent Object Reference") (Other :type "Actor Object Reference") (OtherComp :type "PrimitiveComponent Object Reference") (bSelfMoved :type Boolean) (HitLocation :type "Vector Structure") (HitNormal :type "Vector Structure") (NormalImpulse :type "Vector Structure") (Hit :type "HitResult Structure (by ref)"))
  ; 이펙트 및 사운드
  (`self.PlayFX`)
  (if (`self.ActorHasTag` Other "Enemy")
    ; 적이라면 Overlap이벤트에서 저장했던 배열을 가져와 배열 안의 Actor들에게 TakeDamge함수 실행후 액터 삭제
    (for _array_element (`self.Targets`)
      (bind _asbp_enemy_pawn (cast `/Game/BluePrint/Enemy/BP_EnemyPawn` _array_element))
      (if (`KismetSystemLibrary.IsValid` _asbp_enemy_pawn)
        (`/Game/BluePrint/Enemy/BP_EnemyPawn.TakeDamage` _asbp_enemy_pawn (`self.BulletDamage`))))
    (`self.K2_DestroyActor`)
    (else
      ; 적이 아니라면 액터 삭제
      (`self.K2_DestroyActor`))))

(fn `UserConstructionScript`
  (`parent.UserConstructionScript`))