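; BP_TowerBase is a selectable build spot that the player turns into a Pawn, Rook, Knight or Bishop tower.
; Selecting it spawns a BP_TowerActions actor above it, unselecting destroys that actor, and a separate function toggles its outline highlight.
; A received action deselects the tower and checks the controller's gold against that type's cost.
; Success spawns the tower, deducts gold and destroys the base, while failure fades in the HUD coin banner, each with a sound.
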(event `self.ReceiveBeginPlay`
  (bind _aspc_player_controller (cast `/Game/BluePrint/PC_PlayerController` (`GameplayStatics.GetPlayerController` 0)))
  (set `self.PlayerController` _aspc_player_controller))

(event `/Game/BluePrint/BPI_TowerAction.OnTowerAction`
  (params (TowerAction :type "/Game/BluePrint/Tower/E_TowerAction Enum" :default "NewEnumerator0"))
  ; 위젯에서 받아온 액션을 실행
  (bind _ashud_base_ui (cast `/Game/UI/HUD_BaseUI` (`PlayerController.GetHUD` (`GameplayStatics.GetPlayerController` 0))))
  (set `self.Widget` (`/Game/UI/HUD_BaseUI.BaseWidget` _ashud_base_ui))
  (`self.DoTowerAction` TowerAction))

(fn `DoTowerAction`
  (params (TowerAction :type "/Game/BluePrint/Tower/E_TowerAction Enum" :default "NewEnumerator0"))
  (bind _returnvalue (`self.GetTransform`))
  (`|ExecutionSequence`
    (:`then_0`
      (bind (_isvalid _aspc_player_controller) (`/Game/BluePrint/BPFL_Utility.GetPlayer`))
      ; 액션이 들어오면 타워 선택 해제
      (if _isvalid
        (`/Game/BluePrint/PC_PlayerController.UnSelectTower` _aspc_player_controller)))
    (:`then_1`
      ; 선택에 따라 타워 액션 실행
      (switch `/Game/BluePrint/Tower/E_TowerAction` TowerAction
        (:`NewEnumerator1`
          (`self.BuildPawnTower` _returnvalue))
        (:`NewEnumerator2`
          (`self.BuildRookTower` _returnvalue))
        (:`NewEnumerator3`
          (`self.BuildKnightTower` _returnvalue))
        (:`NewEnumerator4`
          (`self.BuildBishopTower` _returnvalue)))
      ; Base 타워를 제거
      (`self.K2_DestroyActor`))))

(fn `Select`
  ; 선택한 타워에 타워 액션 생성
  (bind _returnvalue (`|SpawnActorFromClass` "/Game/BluePrint/Tower/BP_TowerActions.BP_TowerActions_C" (`KismetMathLibrary.MakeTransform` (+ (`self.K2_GetActorLocation`) (0.0 0.0 100.0))) "Undefined" "MultiplyWithRoot" self "NewEnumerator1" "NewEnumerator2" "NewEnumerator4" "NewEnumerator3" null))
  (set `self.TowerActions` _returnvalue))

(fn `SetHighLight`
  (params (IsHighLighted :type Boolean))
  ; 윤곽선 활성화
  (`SceneComponent.SetVisibility` (`self.HighLight`) IsHighLighted false))

(fn `UnSelect`
  ; 타워 액션을 삭제
  (bind _toweractions (`self.TowerActions`)
    (:`then`
      (`self.K2_DestroyActor` _toweractions)
      (set `self.TowerActions` null))
    (:`else`)))

(fn `UserConstructionScript`)