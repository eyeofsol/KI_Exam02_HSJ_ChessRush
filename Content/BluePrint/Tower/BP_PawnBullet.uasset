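; BP_PawnBullet is a homing tower bullet that damages a targeted enemy pawn.
; On BeginPlay, if a target exists, its projectile movement homes on the first TargetActor's root component and the bullet destroys itself after a short delay.
; On hit, it passes BulletDamage to the target's BP_EnemyPawn TakeDamage and destroys itself; hitting any other actor destroys it without damage.
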(event `self.ReceiveBeginPlay`
  (if (not (`KismetArrayLibrary.Array_IsEmpty` (`self.TargetActor`)))
    (set `ProjectileMovementComponent.HomingTargetComponent` (`Actor.RootComponent` (`|GetArrayItem` (`self.TargetActor`))) (`self.ProjectileMovement`))
    (`KismetSystemLibrary.Delay` 3.0)
    (`self.K2_DestroyActor`)))

(event `self.ReceiveHit`
  (params (MyComp :type "PrimitiveComponent Object Reference") (Other :type "Actor Object Reference") (OtherComp :type "PrimitiveComponent Object Reference") (bSelfMoved :type Boolean) (HitLocation :type "Vector Structure") (HitNormal :type "Vector Structure") (NormalImpulse :type "Vector Structure") (Hit :type "HitResult Structure (by ref)"))
  (if (== Other (`|GetArrayItem` (`self.TargetActor`)))
    (bind _asbp_enemy_pawn (cast `/Game/BluePrint/Enemy/BP_EnemyPawn` Other))
    (`/Game/BluePrint/Enemy/BP_EnemyPawn.TakeDamage` _asbp_enemy_pawn (`self.BulletDamage`))
    (`self.K2_DestroyActor`)
    (else
      (`self.K2_DestroyActor`))))

(fn `UserConstructionScript`)