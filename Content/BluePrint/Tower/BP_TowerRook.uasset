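; BP_TowerRook is the Rook tower, a child tower Blueprint that fires cannonballs and offers an upgrade and sell menu.
; BeginPlay sets its cost, and Attack spawns a BP_CannonBall at FirePoint aimed at the first target, passing on FireDamage.
; Select replaces the parent logic, spawning a BP_RookTowerUpdate menu actor above the tower and showing the range indicator.
; UnSelect destroys that actor and hides the range.
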(event `self.ReceiveBeginPlay`
  (`parent.ReceiveBeginPlay`)
  (set `self.TowerCost` (`self.RookCost`)))

(event `self.Attack`
  (bind _returnvalue (`|SpawnActorFromClass` "/Game/BluePrint/Tower/BP_CannonBall.BP_CannonBall_C" (`SceneComponent.K2_GetComponentToWorld` (`self.FirePoint`)) "Undefined" "MultiplyWithRoot" null (`|GetArrayItem` (`self.Targets`)) null))
  (bind _output_get (set `self.Bullet` _returnvalue))
  (set `/Game/BluePrint/Tower/BP_Bullet.BulletDamage` (`self.FireDamage`) _output_get))

(fn `Select`
  (bind _returnvalue (`|SpawnActorFromClass` "/Game/BluePrint/Tower/BP_RookTowerUpdate.BP_RookTowerUpdate_C" (`KismetMathLibrary.MakeTransform` (+ (`self.K2_GetActorLocation`) (0.0 0.0 100.0))) "Undefined" "MultiplyWithRoot" self "NewEnumerator5" "NewEnumerator6" (`self.UpgradeCost`) (`self.TowerCost`) null))
  (set `self.RookUpdate` _returnvalue)
  (`SceneComponent.SetVisibility` (`self.ShowRange`) true false))

(fn `UnSelect`
  (bind _rookupdate (`self.RookUpdate`)
    (:`then`
      (`self.K2_DestroyActor` _rookupdate)
      (`SceneComponent.SetVisibility` (`self.ShowRange`) false false))
    (:`else`)))

(fn `UserConstructionScript`
  (`parent.UserConstructionScript`))