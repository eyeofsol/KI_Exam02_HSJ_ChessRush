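; BP_TestEnemy is a test enemy that travels along a route spline and costs the player health when it reaches the end.
; Init stores the route actor and places the enemy at the spline's start.
; Tick advances a distance by MoveSpeed and delta time, moving the enemy to that point on the spline.
; Past the spline's end, it decrements Health on the cached PC_PlayerController and destroys itself.
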(event `self.ReceiveBeginPlay`
  (bind _aspc_player_controller (cast `/Game/BluePrint/PC_PlayerController` (`GameplayStatics.GetPlayerController` 0)))
  (set `self.PlayerController` _aspc_player_controller))

(event `self.ReceiveTick`
  (params (DeltaSeconds :type "Float (single-precision)"))
  (bind _playercontroller (`self.PlayerController`))
  (bind _route (`/Game/BluePrint/BP_TestRoute.Route` (`self.MoveRoute`)))
  (bind _output_get (set `self.CurrentDistance` (+ (* DeltaSeconds (`self.MoveSpeed`)) (`self.CurrentDistance`))))
  (if (< _output_get (`SplineComponent.GetSplineLength` _route))
    (`self.K2_SetActorLocation` (`SplineComponent.GetLocationAtDistanceAlongSpline` _route (`self.CurrentDistance`) "World"))
    (else
      (bind _result (`/Engine/EditorBlueprintResources/StandardMacros.DecrementFloat` (`/Game/BluePrint/PC_PlayerController.Health` _playercontroller))
        (:`  `
          (set `/Game/BluePrint/PC_PlayerController.Health` _result _playercontroller)
          (`self.K2_DestroyActor`))))))

(fn `Init`
  (params (Route :type "/Game/BluePrint/BP_TestRoute Object Reference"))
  (`/Engine/EditorBlueprintResources/StandardMacros.IsValid` Route
    (:`Is Valid`
      (set `self.MoveRoute` Route)
      (set `self.CurrentDistance` 0.0)
      (`self.K2_SetActorLocation` (`SplineComponent.GetLocationAtDistanceAlongSpline` (`/Game/BluePrint/BP_TestRoute.Route` (`self.MoveRoute`)) 0.0 "World")))))

(fn `UserConstructionScript`)