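; BP_EnemyBishop is an enemy Blueprint with a periodic skill that makes it undetectable for a short time.
; Tick runs the parent logic, accumulates a cooldown timer, and fires BishopSkill roughly every ten seconds.
; The skill disables the static mesh's collision and applies a hidden material, then restores collision and the base material after a three-second delay.
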(event `self.ReceiveTick`
  (params (DeltaSeconds :type "Float (single-precision)"))
  (`parent.ReceiveTick` DeltaSeconds)
  (bind _output_get (set `self.SkillCoolTime` (+ DeltaSeconds (`self.SkillCoolTime`))))
  (if (> _output_get 10.0)
    ; 쿨타임이 돌아오면 스킬 발동후 초기화
    (`self.BishopSkill`)
    (set `self.SkillCoolTime` 0.0)))

(event `BishopSkill`
  ; 3초 동안 감지 불가 상태 스킬
  (`PrimitiveComponent.SetCollisionEnabled` (`self.StaticMesh`) "NoCollision")
  (`PrimitiveComponent.SetMaterial` (`self.StaticMesh`) 0 "/Game/Materials/HideEnemy_Mtr.HideEnemy_Mtr")
  (`KismetSystemLibrary.Delay` 3.0)
  (`PrimitiveComponent.SetCollisionEnabled` (`self.StaticMesh`) "QueryAndPhysics")
  (`PrimitiveComponent.SetMaterial` (`self.StaticMesh`) 0 "/Game/Materials/BaseEnemy_Mtr.BaseEnemy_Mtr"))

(fn `UserConstructionScript`
  (`parent.UserConstructionScript`))