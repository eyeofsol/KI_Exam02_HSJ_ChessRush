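; Boss bishop enemy Blueprint that periodically teleports forward and is immune to speed debuffs.
; Tick runs the parent logic and accumulates a cooldown, firing BossBishopSkill every few seconds to jump CurrentDistance ahead by a fixed amount.
; An empty TakeSpeedDebuff event blocks slows.
; ReduceHealth damages the PlayerController's health, triggers GameOver when it is depleted, then destroys the boss.
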(event `self.ReceiveTick`
  (params (DeltaSeconds :type "Float (single-precision)"))
  (`parent.ReceiveTick` DeltaSeconds)
  (bind _output_get (set `self.SkillCoolTime` (+ DeltaSeconds (`self.SkillCoolTime`))))
  (if (> _output_get 3.0)
    ; 쿨타임이 돌아오면 스킬 발동후 초기화
    (`self.BossBishopSkill`)
    (set `self.SkillCoolTime` 0.0)))

(event `BossBishopSkill`
  ; 쿨타임마다 순간이동
  (set `self.CurrentDistance` (+ (`self.CurrentDistance`) 500.0)))

(event `self.TakeSpeedDebuff`
  ; 보스는 속도 디버프를 받지 않기 위해 설정
)

(fn `ReduceHealth`
  (bind _playercontroller (`self.PlayerController`))
  (bind _output_get (set `/Game/BluePrint/PC_PlayerController.Health` (- (`/Game/BluePrint/PC_PlayerController.Health` _playercontroller) 10.0) _playercontroller))
  (if (not (> _output_get 0.0))
    (`/Game/BluePrint/PC_PlayerController.GameOver` _playercontroller))
  (`self.K2_DestroyActor`))

(fn `UserConstructionScript`
  (`parent.UserConstructionScript`))