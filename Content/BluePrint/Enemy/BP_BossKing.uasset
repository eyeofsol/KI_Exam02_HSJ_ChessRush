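; King boss enemy, derived from a parent enemy, that summons other bosses and ends the game when killed.
; Tick runs a roughly seven-second cooldown, then asks the level's BP_SpawnManager to spawn a random Rook, Knight or Bishop boss.
; It ignores speed debuffs through an empty event, and its death pauses the game and calls GameOver as the clear condition.
; ReduceHealth also calls GameOver and destroys the King, without pausing.
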(event `self.ReceiveBeginPlay`
  (`parent.ReceiveBeginPlay`)
  ; 보스를 스폰하기 위해 스폰매니저를 가져옴
  (bind _returnvalue (`GameplayStatics.GetActorOfClass` "/Game/BluePrint/Enemy/BP_SpawnManager.BP_SpawnManager_C"))
  (set `self.SpawnManager` _returnvalue))

(event `self.TakeSpeedDebuff`
  ; 보스는 속도 디버프를 받지 않기 위해 설정
)

(event `self.ReceiveTick`
  (params (DeltaSeconds :type "Float (single-precision)"))
  (bind _spawnmanager (`self.SpawnManager`))
  (`parent.ReceiveTick` DeltaSeconds)
  (bind _output_get (set `self.SkillCoolTime` (+ DeltaSeconds (`self.SkillCoolTime`))))
  (if (> _output_get 7.0)
    (switch `int` (`KismetMathLibrary.RandomIntegerInRange` 0 2)
      (:`0`
        ; 쿨타임이 돌아오면 랜덤한 보스 스폰 후 초기화
        (`/Game/BluePrint/Enemy/BP_SpawnManager.SpawnBossRook` _spawnmanager))
      (:`1`
        (`/Game/BluePrint/Enemy/BP_SpawnManager.SpawnBossKnight` _spawnmanager))
      (:`2`
        (`/Game/BluePrint/Enemy/BP_SpawnManager.SpawnBossBishop` _spawnmanager)))
    (set `self.SkillCoolTime` 0.0)))

(event `self.TakeDamage`
  (params (Damage :type "Float (double-precision)"))
  (set `self.CurrentHealth` (- (`self.CurrentHealth`) Damage))
  (`self.UpdateHpBar`)
  (if (<= (`self.CurrentHealth`) 0.0)
    (`self.K2_DestroyActor`)
    ; 게임 클리어 판정
    (`GameplayStatics.SetGamePaused` true)
    (`/Game/BluePrint/PC_PlayerController.GameOver` (`self.PlayerController`))))

(fn `ReduceHealth`
  (`/Game/BluePrint/PC_PlayerController.GameOver` (`self.PlayerController`))
  (`self.K2_DestroyActor`))

(fn `UserConstructionScript`
  (`parent.UserConstructionScript`))