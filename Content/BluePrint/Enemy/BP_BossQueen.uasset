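; BP_BossQueen is a boss enemy that combines the Rook, Knight and Bishop boss skills and ignores speed debuffs.
; On Tick, a cooldown timer periodically fires one at random: a heal capped at max health, a brief speed burst, or a jump in CurrentDistance.
; TakeSpeedDebuff is deliberately empty to give the immunity.
; ReduceHealth damages the player, triggers game over at zero health, and destroys the boss.
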(event `self.TakeSpeedDebuff`
  ; 보스는 속도 디버프를 받지 않기 위해 설정
)

(event `self.ReceiveTick`
  (params (DeltaSeconds :type "Float (single-precision)"))
  (`parent.ReceiveTick` DeltaSeconds)
  (bind _output_get (set `self.SkillCoolTime` (+ DeltaSeconds (`self.SkillCoolTime`))))
  (if (> _output_get 3.0)
    (switch `int` (`KismetMathLibrary.RandomIntegerInRange` 0 2)
      (:`0`
        ; 쿨타임이 돌아오면 랜덤한 스킬 발동후 초기화
        (`self.BossRookSkill`))
      (:`1`
        (`self.BossKnightSkill`))
      (:`2`
        (`self.BossBishopSkill`)))
    (set `self.SkillCoolTime` 0.0)))

(event `BossRookSkill`
  (bind _maxhealth (`self.MaxHealth`))
  (bind _currenthealth (`self.CurrentHealth`))
  ; 룩 보스의 스킬
  (set `self.CurrentHealth` (+ _currenthealth 200.0))
  (`self.UpdateHpBar`)
  (if (> _currenthealth _maxhealth)
    (set `self.CurrentHealth` _maxhealth)))

(event `BossKnightSkill`
  ; 나이트 보스의 스킬
  (set `self.MoveSpeed` (+ (`self.MoveSpeed`) 300.0))
  (`KismetSystemLibrary.Delay` 1.0)
  (set `self.MoveSpeed` (`self.MaxSpeed`)))

(event `BossBishopSkill`
  ; 비숍 보스의 스킬
  (set `self.CurrentDistance` (+ (`self.CurrentDistance`) 500.0)))

(fn `ReduceHealth`
  (bind _playercontroller (`self.PlayerController`))
  (bind _output_get (set `/Game/BluePrint/PC_PlayerController.Health` (- (`/Game/BluePrint/PC_PlayerController.Health` _playercontroller) 10.0) _playercontroller))
  (if (not (> _output_get 0.0))
    (`/Game/BluePrint/PC_PlayerController.GameOver` _playercontroller))
  (`self.K2_DestroyActor`))

(fn `UserConstructionScript`
  (`parent.UserConstructionScript`))