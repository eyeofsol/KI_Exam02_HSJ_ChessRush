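; Enemy pawn that follows a spline route toward the player's goal, with health, a gold reward and a slow debuff.
; Init sets the route, then Tick advances distance along the spline and aligns the transform to it.
; Damage reveals the HP widget and death awards gold, while reaching the end costs player health and can trigger GameOver.
; The debuff cuts speed by a third and swaps to a frozen material, refreshing on reapplication until it expires.
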(event `self.ReceiveBeginPlay`
  ; 생성시 세팅 초기화(Init)
  (bind _aspc_player_controller (cast `/Game/BluePrint/PC_PlayerController` (`GameplayStatics.GetPlayerController` 0)))
  (set `self.PlayerController` _aspc_player_controller)
  (set `self.CurrentHealth` (`self.MaxHealth`))
  (bind _aswbp_enemy_hp (cast `/Game/UI/WBP_EnemyHP` (`WidgetComponent.GetUserWidgetObject` (`self.HPBar`))))
  (bind _output_get (set `self.As WBP Enemy HP` _aswbp_enemy_hp))
  (`Widget.SetVisibility` _output_get "Hidden"))

(event `self.ReceiveTick`
  (params (DeltaSeconds :type "Float (single-precision)"))
  (bind (_ismove _route) (`self.UpdateCurrentDirection` DeltaSeconds))
  ; 목적지 도착 여부
  (if _ismove
    (`self.MoveLocation` _route)
    ; 디버프 상태 체크
    (if (`self.IsDebuff`)
      ; 디버프 상태일때 Debuff Time만큼 시간 경과시 디버프 해제
      (set `self.DebuffDuration` (+ DeltaSeconds (`self.DebuffDuration`)))
      (if (>= (`self.DebuffDuration`) (`self.DebuffTime`))
        (set `self.IsDebuff` false)
        (set `self.MoveSpeed` (`self.MaxSpeed`))
        (`PrimitiveComponent.SetMaterial` (`self.StaticMesh`) 0 "/Game/Materials/BaseEnemy_Mtr.BaseEnemy_Mtr")))
    (else
      ; 플레이어 체력 감소
      (`self.ReduceHealth`))))

(event `TakeDamage`
  (params (Damage :type "Float (double-precision)"))
  (bind _playercontroller (`self.PlayerController`))
  ; 데미지 만큼 현재 체력 감소
  (set `self.CurrentHealth` (- (`self.CurrentHealth`) Damage))
  ; HP바 업데이트 후 죽었는지 체크
  (`self.UpdateHpBar`)
  (if (<= (`self.CurrentHealth`) 0.0)
    ; 죽었다면 플레이어의 골드를 증가시키고 액터 파괴
    (set `/Game/BluePrint/PC_PlayerController.Gold` (+ (`/Game/BluePrint/PC_PlayerController.Gold` _playercontroller) (`self.DropGold`)) _playercontroller)
    (`self.K2_DestroyActor`)))

(event `TakeSpeedDebuff`
  (if (`self.IsDebuff`)
    ; 원래 디버프 상태였다면 디버프 경과시간을 초기화
    (set `self.DebuffDuration` 0.0)
    (else
      (set `self.IsDebuff` true)
      ; 디버프 경과시간을 초기화 하고 이동속도를 절반으로 감소
      (set `self.DebuffDuration` 0.0)
      (set `self.MoveSpeed` (- (`self.MoveSpeed`) (/ (`self.MaxSpeed`) 3.0)))
      (`PrimitiveComponent.SetMaterial` (`self.StaticMesh`) 0 "/Game/Materials/FrozenEnemy_Mtr.FrozenEnemy_Mtr"))))

(fn `Init`
  (params (Route :type "/Game/BluePrint/Enemy/BP_WaveRoute Object Reference"))
  (`/Engine/EditorBlueprintResources/StandardMacros.IsValid` Route
    (:`Is Valid`
      ; 적이 이동할 경로를 전달하고
      ; 이동 속도를 초기화
      (set `self.MoveRoute` Route)
      (set `self.MoveSpeed` (`self.MaxSpeed`))
      ; 이동 루트의 초기 위치로 적의 위치를 설정
      (set `self.CurrentDistance` 0.0)
      (`self.K2_SetActorLocation` (`SplineComponent.GetLocationAtDistanceAlongSpline` (`/Game/BluePrint/Enemy/BP_WaveRoute.Route` (`self.MoveRoute`)) 0.0 "World")))))

(fn `ReduceHealth`
  (bind _playercontroller (`self.PlayerController`))
  ; 플레이어의 체력을 감소시키고 플레이어의 체력이 0보다 작으면 GameOver 이벤트 실행
  (bind _result (`/Engine/EditorBlueprintResources/StandardMacros.DecrementFloat` (`/Game/BluePrint/PC_PlayerController.Health` _playercontroller))
    (:`  `
      (bind _output_get (set `/Game/BluePrint/PC_PlayerController.Health` _result _playercontroller))
      (if (not (> _output_get 0.0))
        (`/Game/BluePrint/PC_PlayerController.GameOver` _playercontroller))
      (`self.K2_DestroyActor`))))

(fn `UpdateHpBar`
  (bind _as_wbp_enemy_hp (`self.As WBP Enemy HP`))
  (set `/Game/UI/WBP_EnemyHP.Percent` (/ (`self.CurrentHealth`) (`self.MaxHealth`)) _as_wbp_enemy_hp)
  (`Widget.SetVisibility` _as_wbp_enemy_hp "Visible"))

(fn `UserConstructionScript`)