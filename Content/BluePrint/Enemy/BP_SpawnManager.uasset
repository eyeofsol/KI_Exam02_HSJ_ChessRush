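; Spawn manager that runs 25 scripted waves of chess-piece enemies and bosses along the BP_WaveRoute spline.
; The HUD play button hides itself and starts a timer on the function name built from "Wave" plus the controller's Wave number.
; Each wave spawns tagged enemies at the spline start through delayed loops.
; When spawning finishes, not when enemies die, WaveEnd increments Wave and reshows the button, except after final Wave25.
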(event `self.ReceiveBeginPlay`
  (bind _hud (`self.Init`))
  (`/Engine/EditorBlueprintResources/StandardMacros.IsValid` (`/Game/UI/HUD_BaseUI.BaseWidget` _hud)
    (:`Is Valid`
      ; 시작 버튼 눌림 바인드
      (add `/Game/UI/WBP_BaseUI.OnPlayButtonPressed` (`/Game/UI/HUD_BaseUI.BaseWidget` (`self.HUD`)) (delegate `OnPlayButtonPressed_이벤트`) :!label _label))
    (:`Is Not Valid`
      ; HUD가 존재하지 않다면 위젯 생성 이벤트 호출
      (add `/Game/UI/HUD_BaseUI.OnWidgetCreated` _hud (delegate `OnWidgetCreated_이벤트`)))))

(event `TestWave`
  ; TestWave 설정
  (`/Game/BluePrint/BP_DelayForLoop.ForLoopDelay` 1 1 2.0
    (:`Completed`
      (`self.SpawnBossKing`)
      (`self.WaveEnd`))))

(event `OnWidgetCreated_이벤트`
  ; HUD가 존재하지 않다면 위젯 생성 이벤트 호출
  (goto _label))

(event `OnPlayButtonPressed_이벤트`
  (`Widget.SetVisibility` (`/Game/UI/WBP_BaseUI.PlayButton` (`/Game/UI/HUD_BaseUI.BaseWidget` (`self.HUD`))) "Hidden")
  (`self.Wave Start`))

(event `Wave Start`
  ; Wave(int)를 활용해 해당 웨이브 이벤트 실행
  (`KismetSystemLibrary.K2_SetTimer` null (`KismetStringLibrary.BuildString_Int` "Wave" "" (`/Game/BluePrint/PC_PlayerController.Wave` (`self.PlayerController`))) 0.1))

(event `Wave1`
  ; 웨이브 정보
  (`self.Wave1Spawn`
    (:`Completed`
      (`self.WaveEnd` :!label _label_2))))

(event `Wave6`
  ; 웨이브 정보
  (`self.Wave6Spawn`
    (:`Completed`
      (`self.WaveEnd` :!label _label_3))))

(event `Wave11`
  ; 웨이브 정보
  (`self.Wave11Spawn`
    (:`Completed`
      (`self.WaveEnd` :!label _label_4))))

(event `Wave2`
  ; 웨이브 정보
  (`self.Wave2Spawn`
    (:`Completed`
      (goto _label_2))))

(event `Wave7`
  ; 웨이브 정보
  (`self.Wave7Spawn`
    (:`Completed`
      (goto _label_3))))

(event `Wave12`
  ; 웨이브 정보
  (`self.Wave12Spawn`
    (:`Completed`
      (goto _label_4))))

(event `Wave3`
  ; 웨이브 정보
  (`self.Wave3Spawn`
    (:`Completed`
      (goto _label_2))))

(event `Wave8`
  ; 웨이브 정보
  (`self.Wave8Spawn`
    (:`Completed`
      (goto _label_3))))

(event `Wave13`
  ; 웨이브 정보
  (`self.Wave13Spawn`
    (:`Completed`
      (goto _label_4))))

(event `Wave4`
  ; 웨이브 정보
  (`self.Wave4Spawn`
    (:`Completed`
      (goto _label_2))))

(event `Wave9`
  ; 웨이브 정보
  (`self.Wave9Spawn`
    (:`Completed`
      (goto _label_3))))

(event `Wave14`
  ; 웨이브 정보
  (`self.Wave14Spawn`
    (:`Completed`
      (goto _label_4))))

(event `Wave5`
  ; 웨이브 정보
  (`self.Wave5Spawn`
    (:`Completed`
      (goto _label_2))))

(event `Wave10`
  ; 웨이브 정보
  (`self.Wave10Spawn`
    (:`Completed`
      (goto _label_3))))

(event `Wave15`
  ; 웨이브 정보
  (`self.Wave15Spawn`
    (:`Completed`
      (goto _label_4))))

(event `Wave16`
  ; 웨이브 정보
  (`self.Wave16Spawn`
    (:`Completed`
      (`self.WaveEnd` :!label _label_5))))

(event `Wave21`
  ; 웨이브 정보
  (`self.Wave21Spawn`
    (:`Completed`
      (`self.WaveEnd` :!label _label_6))))

(event `Wave17`
  ; 웨이브 정보
  (`self.Wave17Spawn`
    (:`Completed`
      (goto _label_5))))

(event `Wave22`
  ; 웨이브 정보
  (`self.Wave22Spawn`
    (:`Completed`
      (goto _label_6))))

(event `Wave18`
  ; 웨이브 정보
  (`self.Wave18Spawn`
    (:`Completed`
      (goto _label_5))))

(event `Wave23`
  ; 웨이브 정보
  (`self.Wave23Spawn`
    (:`Completed`
      (goto _label_6))))

(event `Wave19`
  ; 웨이브 정보
  (`self.Wave19Spawn`
    (:`Completed`
      (goto _label_5))))

(event `Wave24`
  ; 웨이브 정보
  (`self.Wave24Spawn`
    (:`Completed`
      (goto _label_6))))

(event `Wave20`
  ; 웨이브 정보
  (`self.Wave20Spawn`
    (:`Completed`
      (goto _label_5))))

(event `Wave25`
  ; 웨이브 정보
  (`self.Wave25Spawn`))

(fn `SpawnBishop`
  (bind _returnvalue (`GameplayStatics.GetActorOfClass` "/Game/BluePrint/Enemy/BP_WaveRoute.BP_WaveRoute_C"))
  (bind _returnvalue_2 (`|SpawnActorFromClass` "/Game/BluePrint/Enemy/BP_EnemyBishop.BP_EnemyBishop_C" (`KismetMathLibrary.Conv_VectorToTransform` (`SplineComponent.GetLocationAtDistanceAlongSpline` (`/Game/BluePrint/Enemy/BP_WaveRoute.Route` _returnvalue) 0.0 "World")) "Undefined" "MultiplyWithRoot" null null))
  (`KismetArrayLibrary.Array_Add` (`Actor.Tags` _returnvalue_2) "Enemy")
  (`/Game/BluePrint/Enemy/BP_EnemyPawn.Init` _returnvalue_2 _returnvalue))

(fn `SpawnBossBishop`
  (bind _returnvalue (`GameplayStatics.GetActorOfClass` "/Game/BluePrint/Enemy/BP_WaveRoute.BP_WaveRoute_C"))
  (bind _returnvalue_2 (`|SpawnActorFromClass` "/Game/BluePrint/Enemy/BP_BossBishop.BP_BossBishop_C" (`KismetMathLibrary.Conv_VectorToTransform` (`SplineComponent.GetLocationAtDistanceAlongSpline` (`/Game/BluePrint/Enemy/BP_WaveRoute.Route` _returnvalue) 0.0 "World")) "Undefined" "MultiplyWithRoot" null null))
  (`KismetArrayLibrary.Array_Add` (`Actor.Tags` _returnvalue_2) "Enemy")
  (`/Game/BluePrint/Enemy/BP_EnemyPawn.Init` _returnvalue_2 _returnvalue))

(fn `SpawnBossKing`
  (bind _returnvalue (`GameplayStatics.GetActorOfClass` "/Game/BluePrint/Enemy/BP_WaveRoute.BP_WaveRoute_C"))
  (bind _returnvalue_2 (`|SpawnActorFromClass` "/Game/BluePrint/Enemy/BP_BossKing.BP_BossKing_C" (`KismetMathLibrary.Conv_VectorToTransform` (`SplineComponent.GetLocationAtDistanceAlongSpline` (`/Game/BluePrint/Enemy/BP_WaveRoute.Route` _returnvalue) 0.0 "World")) "Undefined" "MultiplyWithRoot" null null))
  (`KismetArrayLibrary.Array_Add` (`Actor.Tags` _returnvalue_2) "Enemy")
  (`/Game/BluePrint/Enemy/BP_EnemyPawn.Init` _returnvalue_2 _returnvalue))

(fn `SpawnBossKnight`
  (bind _returnvalue (`GameplayStatics.GetActorOfClass` "/Game/BluePrint/Enemy/BP_WaveRoute.BP_WaveRoute_C"))
  (bind _returnvalue_2 (`|SpawnActorFromClass` "/Game/BluePrint/Enemy/BP_BossKnight.BP_BossKnight_C" (`KismetMathLibrary.Conv_VectorToTransform` (`SplineComponent.GetLocationAtDistanceAlongSpline` (`/Game/BluePrint/Enemy/BP_WaveRoute.Route` _returnvalue) 0.0 "World")) "Undefined" "MultiplyWithRoot" null null))
  (`KismetArrayLibrary.Array_Add` (`Actor.Tags` _returnvalue_2) "Enemy")
  (`/Game/BluePrint/Enemy/BP_EnemyPawn.Init` _returnvalue_2 _returnvalue))

(fn `SpawnBossQueen`
  (bind _returnvalue (`GameplayStatics.GetActorOfClass` "/Game/BluePrint/Enemy/BP_WaveRoute.BP_WaveRoute_C"))
  (bind _returnvalue_2 (`|SpawnActorFromClass` "/Game/BluePrint/Enemy/BP_BossQueen.BP_BossQueen_C" (`KismetMathLibrary.Conv_VectorToTransform` (`SplineComponent.GetLocationAtDistanceAlongSpline` (`/Game/BluePrint/Enemy/BP_WaveRoute.Route` _returnvalue) 0.0 "World")) "Undefined" "MultiplyWithRoot" null null))
  (`KismetArrayLibrary.Array_Add` (`Actor.Tags` _returnvalue_2) "Enemy")
  (`/Game/BluePrint/Enemy/BP_EnemyPawn.Init` _returnvalue_2 _returnvalue))

(fn `SpawnBossRook`
  (bind _returnvalue (`GameplayStatics.GetActorOfClass` "/Game/BluePrint/Enemy/BP_WaveRoute.BP_WaveRoute_C"))
  (bind _returnvalue_2 (`|SpawnActorFromClass` "/Game/BluePrint/Enemy/BP_BossRook.BP_BossRook_C" (`KismetMathLibrary.Conv_VectorToTransform` (`SplineComponent.GetLocationAtDistanceAlongSpline` (`/Game/BluePrint/Enemy/BP_WaveRoute.Route` _returnvalue) 0.0 "World")) "Undefined" "MultiplyWithRoot" null null))
  (`KismetArrayLibrary.Array_Add` (`Actor.Tags` _returnvalue_2) "Enemy")
  (`/Game/BluePrint/Enemy/BP_EnemyPawn.Init` _returnvalue_2 _returnvalue))

(fn `SpawnKnight`
  (bind _returnvalue (`GameplayStatics.GetActorOfClass` "/Game/BluePrint/Enemy/BP_WaveRoute.BP_WaveRoute_C"))
  (bind _returnvalue_2 (`|SpawnActorFromClass` "/Game/BluePrint/Enemy/BP_EnemyKnight.BP_EnemyKnight_C" (`KismetMathLibrary.Conv_VectorToTransform` (`SplineComponent.GetLocationAtDistanceAlongSpline` (`/Game/BluePrint/Enemy/BP_WaveRoute.Route` _returnvalue) 0.0 "World")) "Undefined" "MultiplyWithRoot" null null))
  (`KismetArrayLibrary.Array_Add` (`Actor.Tags` _returnvalue_2) "Enemy")
  (`/Game/BluePrint/Enemy/BP_EnemyPawn.Init` _returnvalue_2 _returnvalue))

(fn `SpawnPawn`
  (bind _returnvalue (`GameplayStatics.GetActorOfClass` "/Game/BluePrint/Enemy/BP_WaveRoute.BP_WaveRoute_C"))
  (bind _returnvalue_2 (`|SpawnActorFromClass` "/Game/BluePrint/Enemy/BP_EnemyPawn.BP_EnemyPawn_C" (`KismetMathLibrary.Conv_VectorToTransform` (`SplineComponent.GetLocationAtDistanceAlongSpline` (`/Game/BluePrint/Enemy/BP_WaveRoute.Route` _returnvalue) 0.0 "World")) "Undefined" "MultiplyWithRoot" null null))
  (`KismetArrayLibrary.Array_Add` (`Actor.Tags` _returnvalue_2) "Enemy")
  (`/Game/BluePrint/Enemy/BP_EnemyPawn.Init` _returnvalue_2 _returnvalue))

(fn `SpawnRook`
  (bind _returnvalue (`GameplayStatics.GetActorOfClass` "/Game/BluePrint/Enemy/BP_WaveRoute.BP_WaveRoute_C"))
  (bind _returnvalue_2 (`|SpawnActorFromClass` "/Game/BluePrint/Enemy/BP_EnemyRook.BP_EnemyRook_C" (`KismetMathLibrary.Conv_VectorToTransform` (`SplineComponent.GetLocationAtDistanceAlongSpline` (`/Game/BluePrint/Enemy/BP_WaveRoute.Route` _returnvalue) 0.0 "World")) "Undefined" "MultiplyWithRoot" null null))
  (`KismetArrayLibrary.Array_Add` (`Actor.Tags` _returnvalue_2) "Enemy")
  (`/Game/BluePrint/Enemy/BP_EnemyPawn.Init` _returnvalue_2 _returnvalue))

(fn `UserConstructionScript`)

(fn `WaveEnd`
  (bind _playercontroller (`self.PlayerController`))
  (bind _result (`/Engine/EditorBlueprintResources/StandardMacros.IncrementInt` (`/Game/BluePrint/PC_PlayerController.Wave` _playercontroller))
    (:`  `
      (set `/Game/BluePrint/PC_PlayerController.Wave` _result _playercontroller)
      (`Widget.SetVisibility` (`/Game/UI/WBP_BaseUI.PlayButton` (`/Game/UI/HUD_BaseUI.BaseWidget` (`self.HUD`))) "Visible"))))