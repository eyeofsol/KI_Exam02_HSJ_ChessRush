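; BP_TowerPawn is a tower that fires bullets at Enemy-tagged actors in its ShotRange.
; Range overlaps maintain a target list, and each tick FirePoint rotates toward the first entry.
; A looping timer at FireRate spawns BP_PawnBullet from FirePoint, passing the targets and FireDamage.
; Any begin overlap starts the timer if idle, and any end overlap stops it, even if targets remain.
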(event `self.ReceiveTick`
  (params (DeltaSeconds :type "Float (single-precision)"))
  (`self.SetTargetRotation`))

(event `self.ShotRange.OnComponentBeginOverlap`
  (params (OverlappedComponent :type "PrimitiveComponent Object Reference") (OtherActor :type "Actor Object Reference") (OtherComp :type "PrimitiveComponent Object Reference") (OtherBodyIndex :type Integer) (bFromSweep :type Boolean) (SweepResult :type "HitResult Structure (by ref)"))
  (`self.AddTarget` OtherActor)
  (if (not (`self.bIsFire`))
    (bind _returnvalue (`KismetSystemLibrary.K2_SetTimerDelegate` (`|CreateDelegate` :!event `Attack`) (`self.FireRate`) true))
    (set `self.FireTimer` _returnvalue)
    (set `self.bIsFire` true)))

(event `self.ShotRange.OnComponentEndOverlap`
  (params (OverlappedComponent :type "PrimitiveComponent Object Reference") (OtherActor :type "Actor Object Reference") (OtherComp :type "PrimitiveComponent Object Reference") (OtherBodyIndex :type Integer))
  (`self.RemoveTarget` OtherActor)
  (`KismetSystemLibrary.K2_ClearAndInvalidateTimerHandle` (`self.FireTimer`))
  (set `self.bIsFire` false))

(event `Attack`
  (bind _returnvalue (`|SpawnActorFromClass` "/Game/BluePrint/BP_PawnBullet.BP_PawnBullet_C" (`SceneComponent.K2_GetComponentToWorld` (`self.FirePoint`)) "Undefined" "MultiplyWithRoot" null (`self.Targets`) null))
  (bind _output_get (set `self.Bullet` _returnvalue))
  (set `/Game/BluePrint/BP_PawnBullet.BulletDamage` (`self.FireDamage`) _output_get))

(fn `UserConstructionScript`)