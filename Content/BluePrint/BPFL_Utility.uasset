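; Blueprint function library with shared helpers for reaching towers and the local player controller.
; GetTowerUnderMouse runs a complex cursor trace from player 0's controller against a single object type and casts the hit actor to BP_TowerBase.
; GetPlayer casts player 0's controller to PC_PlayerController.
; Both return a success flag alongside the typed reference, and both assume a single local player.
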(fn `GetPlayer`
  (returns (IsValid :type Boolean) (`AsPC Player Controller` :type "/Game/BluePrint/PC_PlayerController Object Reference"))
  (bind _aspc_player_controller (cast `/Game/BluePrint/PC_PlayerController` (`GameplayStatics.GetPlayerController` null))
    (:`then`
      (return true _aspc_player_controller))
    (:`CastFailed`
      (return false null))))

(fn `GetTowerUnderMouse`
  (returns (IsFound :type Boolean) (Tower :type "/Game/BluePrint/Tower/BP_TowerBase Object Reference"))
  (bind (_hitresult _returnvalue) (`PlayerController.GetHitResultUnderCursorForObjects` (`GameplayStatics.GetPlayerController` null) (`|MakeArray` "ObjectTypeQuery7" :!type "EObjectTypeQuery Enum") true))
  (if _returnvalue
    (bind _asbp_tower_base (cast `/Game/BluePrint/Tower/BP_TowerBase` (`.HitActor` (`GameplayStatics.BreakHitResult` _hitresult)))
      (:`then`
        (return true _asbp_tower_base))
      (:`CastFailed`
        (return false null)))
    (else
      (return false null))))