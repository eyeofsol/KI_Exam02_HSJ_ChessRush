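; BP_TestBullet is a test projectile that damages enemies it hits.
; On BeginPlay, if TargetActor is not empty, it sets the first actor's root component as the homing target of its ProjectileMovement.
; On Hit, it casts the other actor to BP_TestEnemy, applies BulletDamage through TakeDamage and destroys itself.
; Hits on any other actor are ignored, so the bullet is not destroyed by them.
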(event `self.ReceiveBeginPlay`
  (if (not (`KismetArrayLibrary.Array_IsEmpty` (`self.TargetActor`)))
    (set `ProjectileMovementComponent.HomingTargetComponent` (`Actor.RootComponent` (`|GetArrayItem` (`self.TargetActor`))) (`self.ProjectileMovement`))))

(event `self.ReceiveHit`
  (params (MyComp :type "PrimitiveComponent Object Reference") (Other :type "Actor Object Reference") (OtherComp :type "PrimitiveComponent Object Reference") (bSelfMoved :type Boolean) (HitLocation :type "Vector Structure") (HitNormal :type "Vector Structure") (NormalImpulse :type "Vector Structure") (Hit :type "HitResult Structure (by ref)"))
  (bind _asbp_test_enemy (cast `/Game/BluePrint/BP_TestEnemy` Other))
  (`/Game/BluePrint/BP_TestEnemy.TakeDamage` _asbp_test_enemy (`self.BulletDamage`))
  (`self.K2_DestroyActor`))

(fn `UserConstructionScript`)