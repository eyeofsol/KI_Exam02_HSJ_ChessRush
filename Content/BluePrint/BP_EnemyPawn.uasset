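; Enemy pawn that walks a spline route, as in a tower defense, costing the player health if it reaches the end.
; Init assigns the route, then Tick advances distance by MoveSpeed and sets the location along the spline.
; TakeDamage lowers health, which Tick polls to update the HP bar widget.
; At zero health it adds DropGold to the player controller and destroys itself.
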(event `self.ReceiveBeginPlay`
  (bind _aspc_player_controller (cast `/Game/BluePrint/PC_PlayerController` (`GameplayStatics.GetPlayerController` 0)))
  (set `self.PlayerController` _aspc_player_controller)
  (set `self.CurrentHealth` (`self.MaxHealth`))
  (bind _aswbp_enemy_hp (cast `/Game/UI/WBP_EnemyHP` (`WidgetComponent.GetUserWidgetObject` (`self.HPBar`))))
  (set `self.As WBP Enemy HP` _aswbp_enemy_hp))

(event `self.ReceiveTick`
  (params (DeltaSeconds :type "Float (single-precision)"))
  (bind _playercontroller (`self.PlayerController`))
  (bind (_ismove _route) (`self.UpdateCurrentDirection` DeltaSeconds))
  (if _ismove
    (`self.MoveLocation` _route)
    (`self.UpdateHPBar`)
    (if (<= (`self.CurrentHealth`) 0.0)
      (set `/Game/BluePrint/PC_PlayerController.Gold` (+ (`/Game/BluePrint/PC_PlayerController.Gold` _playercontroller) (`self.DropGold`)) _playercontroller)
      (`self.K2_DestroyActor`))
    (else
      (`self.ArriveLocation`))))

(event `TakeDamage`
  (params (Damage :type "Float (double-precision)"))
  (set `self.CurrentHealth` (- (`self.CurrentHealth`) Damage)))

(fn `Init`
  (params (Route :type "/Game/BluePrint/BP_TestRoute Object Reference"))
  (`/Engine/EditorBlueprintResources/StandardMacros.IsValid` Route
    (:`Is Valid`
      (set `self.MoveRoute` Route)
      (set `self.CurrentDistance` 0.0)
      (`self.K2_SetActorLocation` (`SplineComponent.GetLocationAtDistanceAlongSpline` (`/Game/BluePrint/BP_TestRoute.Route` (`self.MoveRoute`)) 0.0 "World")))))

(fn `UserConstructionScript`)