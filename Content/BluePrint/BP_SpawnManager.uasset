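; BP_SpawnManager runs enemy waves started by the HUD's Play button.
; It binds to the button event on BeginPlay, or waits for the HUD's widget-created event if the widget is not yet valid.
; Each wave hides the button and uses a delayed loop to spawn tagged BP_EnemyPawns at the BP_WaveRoute spline start, initializing each with that route.
; When spawning completes, it increments the PlayerController's Wave and reshows the button.
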(event `self.ReceiveBeginPlay`
  (bind _returnvalue (`GameplayStatics.GetPlayerController` 0))
  (bind _aspc_player_controller (cast `/Game/BluePrint/PC_PlayerController` _returnvalue))
  (set `self.PlayerController` _aspc_player_controller)
  (bind _ashud_base_ui (cast `/Game/UI/HUD_BaseUI` (`PlayerController.GetHUD` _returnvalue)))
  (bind _output_get (set `self.HUD` _ashud_base_ui))
  (`/Engine/EditorBlueprintResources/StandardMacros.IsValid` (`/Game/UI/HUD_BaseUI.BaseWidget` _output_get)
    (:`Is Valid`
      (add `/Game/UI/WBP_BaseUI.OnPlayButtonPressed` (`/Game/UI/HUD_BaseUI.BaseWidget` (`self.HUD`)) (delegate `OnPlayButtonPressed_이벤트`) :!label _label))
    (:`Is Not Valid`
      (add `/Game/UI/HUD_BaseUI.OnWidgetCreated` _output_get (delegate `OnWidgetCreated_이벤트`)))))

(event `OnWidgetCreated_이벤트`
  (goto _label))

(event `OnPlayButtonPressed_이벤트`
  (`Widget.SetVisibility` (`/Game/UI/WBP_BaseUI.PlayButton` (`/Game/UI/HUD_BaseUI.BaseWidget` (`self.HUD`))) "Hidden")
  (`self.Wave Start`))

(event `Wave Start`
  (bind _playercontroller (`self.PlayerController`))
  (`/Game/BluePrint/BP_DelayForLoop.ForLoopDelay` 1 (`self.WaveEnemy`) (`self.DelayTime`)
    (:`LoopBody`
      (`self.SpawnPawn`))
    (:`Completed`
      (bind _result (`/Engine/EditorBlueprintResources/StandardMacros.IncrementInt` (`/Game/BluePrint/PC_PlayerController.Wave` _playercontroller))
        (:`  `
          (set `/Game/BluePrint/PC_PlayerController.Wave` _result _playercontroller)
          (`Widget.SetVisibility` (`/Game/UI/WBP_BaseUI.PlayButton` (`/Game/UI/HUD_BaseUI.BaseWidget` (`self.HUD`))) "Visible"))))))

(fn `SpawnPawn`
  (bind _returnvalue (`GameplayStatics.GetActorOfClass` "/Game/BluePrint/Enemy/BP_WaveRoute.BP_WaveRoute_C"))
  (bind _returnvalue_2 (`|SpawnActorFromClass` "/Game/BluePrint/Enemy/BP_EnemyPawn.BP_EnemyPawn_C" (`KismetMathLibrary.Conv_VectorToTransform` (`SplineComponent.GetLocationAtDistanceAlongSpline` (`/Game/BluePrint/Enemy/BP_WaveRoute.Route` _returnvalue) 0.0 "World")) "Undefined" "MultiplyWithRoot" null null))
  (`KismetArrayLibrary.Array_Add` (`Actor.Tags` _returnvalue_2) "Enemy")
  (`/Game/BluePrint/Enemy/BP_EnemyPawn.Init` _returnvalue_2 _returnvalue))

(fn `UserConstructionScript`)