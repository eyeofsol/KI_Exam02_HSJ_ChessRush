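; BP_TestTower is a tower that fires BP_TestBullet projectiles at actors tagged Enemy within its ShotRange.
; Overlap events maintain the Targets list, starting a looping FireRate timer on the first enemy and clearing it when the list empties.
; The Attack event spawns a bullet at FirePoint and hands it Targets as its TargetActor.
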(event `self.ShotRange.OnComponentBeginOverlap`
  (params (OverlappedComponent :type "PrimitiveComponent Object Reference") (OtherActor :type "Actor Object Reference") (OtherComp :type "PrimitiveComponent Object Reference") (OtherBodyIndex :type Integer) (bFromSweep :type Boolean) (SweepResult :type "HitResult Structure (by ref)"))
  (if (`KismetSystemLibrary.IsValid` OtherActor)
    (if (`self.ActorHasTag` OtherActor "Enemy")
      (`KismetArrayLibrary.Array_Add` (`self.Targets`) OtherActor)
      (if (not (`self.bIsFire`))
        (bind _returnvalue (`KismetSystemLibrary.K2_SetTimerDelegate` (`|CreateDelegate` :!event `Attack`) (`self.FireRate`) true))
        (set `self.bIsFire` true)))))

(event `self.ShotRange.OnComponentEndOverlap`
  (params (OverlappedComponent :type "PrimitiveComponent Object Reference") (OtherActor :type "Actor Object Reference") (OtherComp :type "PrimitiveComponent Object Reference") (OtherBodyIndex :type Integer))
  (bind _targets (`self.Targets`))
  (`KismetArrayLibrary.Array_RemoveItem` _targets OtherActor)
  (if (`KismetArrayLibrary.Array_IsEmpty` _targets)
    (`KismetSystemLibrary.K2_ClearAndInvalidateTimerHandle` (stale `self.ShotRange.OnComponentBeginOverlap` _returnvalue))
    (set `self.bIsFire` false)))

(event `Attack`
  (`|SpawnActorFromClass` "/Game/BluePrint/BP_TestBullet.BP_TestBullet_C" (`SceneComponent.K2_GetComponentToWorld` (`self.FirePoint`)) "Undefined" "MultiplyWithRoot" null (`self.Targets`) null))

(fn `UserConstructionScript`)